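; Enemy spawner actor with a player-triggered TriggerBox and a construction script that labels its debug text.
; A tagged player entering the box starts a fast looping timer; InfiniteFixedWave prunes invalid EnemyPool entries and spawns one BP_Enemy at SpawnPoint while below EnemiesToSpawn, passing AutoAgroPlayer.
; SpawnSmart and SpawnBrainDead spawn single enemies at the actor, the latter stopping its StateTree logic.
; An older delayed burst-spawn branch is left unconnected.
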(event OnComponentBeginOverlap(TriggerBox)
  (params (OverlappedComponent :type Primitive%20Component%20Object%20Reference) (OtherActor :type Actor%20Object%20Reference) (OtherComp :type Primitive%20Component%20Object%20Reference) (OtherBodyIndex :type Integer) (bFromSweep :type Boolean) (SweepResult :type Hit%20Result%20Structure%20%28by%20ref%29))
  (if (Actor|ActorHasTag OtherActor "Player")
    (Utilities|Time|SetTimerbyEvent (EventDispatchers|CreateEvent :!event Custom|InfiniteFixedWave) 0.1 true)))

(event Custom|SpawnSmart
  (Game|SpawnActorfromClass "/Game/Gameplay/AI/BP_Enemy.BP_Enemy_C" (Math|Transform|MakeTransform (Transformation|GetActorLocation) (Math|Rotator|MakeRotator 0.0 0.0 (Math|Random|RandomFloatinRange -9e+01 9e+01)) "1.000000,1.000000,1.000000") "Undefined" "MultiplyWithRoot" 0 false 0))

(event Custom|SpawnBrainDead
  (bind _returnvalue (Game|SpawnActorfromClass "/Game/Gameplay/AI/BP_Enemy.BP_Enemy_C" (Math|Transform|MakeTransform (Transformation|GetActorLocation) (Math|Rotator|MakeRotator 0.0 0.0 (Math|Random|RandomFloatinRange -9e+01 9e+01)) "1.000000,1.000000,1.000000") "Undefined" "MultiplyWithRoot" 0 false 0))
  (bind _asaic_enemy (Utilities|Casting|CastToAIC_Enemy (AI|GetAIController _returnvalue)))
  (AI|Logic|StopLogic (Variables|/Game/Gameplay/AI/AIC_Enemy.AIC_Enemy_C|GetStateTreeAI _asaic_enemy) ""))

(event Custom|InfiniteFixedWave
  (bind _enemypool (Variables|SpawnDetails|GetEnemyPool))
  (for (_array_element _array_index) _enemypool
    (Utilities|IsValid _array_element
      (:Is%20Not%20Valid
        (Utilities|Array|RemoveIndex _enemypool _array_index))))
  (if (< (Utilities|Array|Length (Variables|SpawnDetails|GetEnemyPool)) (Variables|SpawnDetails|GetEnemiesToSpawn))
    (bind _returnvalue (Game|SpawnActorfromClass "/Game/Gameplay/AI/BP_Enemy.BP_Enemy_C" (Math|Transform|MakeTransform (Transformation|GetWorldLocation (Variables|Default|GetSpawnPoint)) (Math|Rotator|MakeRotator 0.0 0.0 (Math|Random|RandomFloatinRange -9e+01 9e+01)) "1.000000,1.000000,1.000000") "AdjustIfPossibleButAlwaysSpawn" "MultiplyWithRoot" 0 (Variables|SpawnDetails|GetAutoAgroPlayer) 0))
    (Utilities|Array|Add (Variables|SpawnDetails|GetEnemyPool) _returnvalue)))

(event Collision|EventActorBeginOverlap
  (params (OtherActor :type Actor%20Object%20Reference)))

(event EventTick
  (params (DeltaSeconds :type Float%20%28single-precision%29)))

(fn ConstructionScript
  (Rendering|Components|TextRender|SetText (Variables|Default|GetDangerZone) (Utilities|Text|ToText(String) (Utilities|String|Append (Variables|Default|GetDebugText) " | Enemies : " (Utilities|String|ToString(Integer) (Variables|SpawnDetails|GetEnemiesToSpawn)))))
  (Rendering|Components|TextRender|SetText (Variables|Default|GetSpawnPointDebug) (Utilities|Text|ToText(String) (Utilities|String|Append "Spawn Point : " (Utilities|GetDisplayName self)))))