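; Wave manager actor that runs sequential enemy waves, updating the HUD and signalling game end after the last.
; Each async-loaded wave tops up a BP_Enemy pool to its cap, then teleports pooled enemies to line-traced positions in random trigger boxes or spawn points.
; A looping timer handles spawning at the cap.
; Once a wave finishes spawning, the next starts after a delay or early clear, enraging survivors.
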(event Custom|OnEnemyDestroyed
  (params (DestroyedActor :type Actor%20Object%20Reference)))

(event Custom|BeginWave
  (bind _outactors (Actor|GetAllActorsOfClass "/Game/Gameplay/AI/Spawn/BP_SpawnPoint.BP_SpawnPoint_C"))
  (Variables|Default|SetSpawnPoints _outactors)
  (Spawners|CloseSpawnPoints)
  (CallFunction|SetupNewWave true false))

(event Custom|ResetDefferedStartWave
  (Utilities|Time|ClearandInvalidateTimerbyHandle (Variables|Deffered|GetStartWaveDeffered)))

(event Custom|MenuStart
  (if (and (stale EventBeginPlay _continue) (Variables|Default|GetAutoStart))
    (Utilities|FlowControl|DelayUntilNextTick)
    (bind _asbp_fps_character (Utilities|Casting|CastToBP_FPS_Character (Game|Player|GetPlayerPawn 0))
      (:then
        (Variables|Default|SetHUD (Variables|/Game/Gameplay/Player/BP_FPS_Character.BP_FPS_Character_C|GetWBP_HUD _asbp_fps_character)))
      (:CastFailed
        (Development|PrintString "failed cast")))
    (bind _outactors (Actor|GetAllActorsOfClass "/Game/Gameplay/AI/Spawn/BP_SpawnPoint.BP_SpawnPoint_C"))
    (Variables|Default|SetSpawnPoints _outactors)
    (Spawners|CloseSpawnPoints)
    (CallFunction|SetupNewWave true false)))

(event Custom|PreSpawningEnemies
  (if (< (Utilities|Array|Length (Variables|Pool|GetEnemies)) (Variables|CurrentWave|GetCurrentWaveMaxCap))
    (Pool|PreSpawnEnemy)
    (Utilities|FlowControl|Delay 0.2)
    (CallFunction|PreSpawningEnemies)))

(event Custom|EndlessSpawn)

(event Custom|ResetDefferedSpawnTimer
  (Utilities|Time|ClearandInvalidateTimerbyHandle (Variables|Deffered|GetSpawnDefferedTimer)))

(event Custom|SetupNewWave
  (params (FirstWave :type Boolean) (DebugForceInstantStart :type Boolean))
  (bind _waves (Variables|Default|GetWaves))
  ;[0.15 0.15 0.15 0.5] Comment
  (if (not (== (Utilities|Array|Length (Variables|Default|GetWaves)) (+ (Variables|Default|GetWaveIndex) 1)))
    (Variables|Default|SetWaveIndex (Math|Integer|SelectInt 0 (+ (Variables|Default|GetWaveIndex) 1) FirstWave))
    (Variables|Deffered|SetForcedStart false)
    (Variables|CurrentWave|SetCurrentWaveSpawnedEnemies 0)
    (if (Utilities|Array|IsValidIndex _waves (Variables|Default|GetWaveIndex))
      (bind _object (Utilities|AsyncLoadAsset (Utilities|Array|Get(acopy) _waves (Variables|Default|GetWaveIndex)))
        (:Completed
          (Utilities|IsValid _object
            (:Is%20Valid
              (bind _output_get (Variables|CurrentWave|SetCurrentWave (Utilities|ResolveSoftReference (Utilities|Array|Get(acopy) _waves (Variables|Default|GetWaveIndex)))))
              (Variables|CurrentWave|SetCurrentWaveMaxCap (Variables|/Game/Gameplay/AI/Spawn/Waves/PDA_WaveData.PDA_WaveData_C|GetMaxEnemyCap _output_get))
              (CallFunction|PreSpawningEnemies)
              (Utilities|FlowControl|Delay 0.2)
              (if DebugForceInstantStart
                (CallFunction|ResetDefferedStartWave :!label _label)
                (CallFunction|ExtractPriorities)
                (CallFunction|DoesWaveHasZonesorBoxes)
                (Spawners|CloseSpawnPoints)
                (Utilities|FlowControl|Sequence
                  (:then_0
                    (CallFunction|EnrageAliveEnemies)
                    (Audio|PlaySound2D (Variables|Default|GetBeginWaveCue) 0.5 1.0 11.0 0 0)
                    (Utilities|FlowControl|Delay 2.0)
                    (Spawners|OpenSpawnPoints)
                    (Development|PrintString (Utilities|String|Append "NEW WAVE : " (Utilities|String|ToString(Integer) (Variables|Default|GetWaveIndex))) true true "(R=1.000000,G=0.000000,B=0.022609,A=1.000000)" 1e+01))
                  (:then_1
                    (Utilities|FlowControl|Delay 4.0)
                    (CallFunction|PickRandomSpawnPoint)))
                (elif (!= (Variables|/Game/Gameplay/AI/Spawn/Waves/PDA_WaveData.PDA_WaveData_C|GetDelayToStart (Variables|CurrentWave|GetCurrentWave)) 0.0)
                  (Utilities|FlowControl|Sequence
                    (:then_0
                      (Default|SetWaveDelay (Variables|Default|GetHUD) (Variables|/Game/Gameplay/AI/Spawn/Waves/PDA_WaveData.PDA_WaveData_C|GetDelayToStart (Variables|CurrentWave|GetCurrentWave)))
                      (Utilities|FlowControl|RetriggerableDelay (Variables|/Game/Gameplay/AI/Spawn/Waves/PDA_WaveData.PDA_WaveData_C|GetDelayToStart (Variables|CurrentWave|GetCurrentWave)))
                      (if (not (Variables|Deffered|GetForcedStart))
                        (goto _label)))
                    (:then_1
                      (if (not (Utilities|Time|IsValidTimerHandle (Variables|Deffered|GetStartWaveDeffered)))
                        (bind _returnvalue (Utilities|Time|SetTimerbyEvent (EventDispatchers|CreateEvent :!event Custom|DefferedStartWave) 1.0 true true))
                        (Variables|Deffered|SetStartWaveDeffered _returnvalue))))
                  (else
                    (goto _label)))))
            (:Is%20Not%20Valid
              (Utilities|Debugging|RaiseScriptError "Last Wave Ended : Path to endless mode" :!label _label_2)))))
      (else
        (goto _label_2)))
    (else
      (Utilities|Debugging|RaiseScriptError "Last wave reached"))))

(event Custom|ResetGatesForSpawn
  (bind (_randomzone _zoneindex) (CallFunction|PickRandomZone))
  (bind (_randompoint _pointindex) (CallFunction|PickRandomPoint))
  (Utilities|FlowControl|Sequence
    (:then_0
      (Utilities|FlowControl|DoOnce false) ; enters at Reset
    )
    (:then_1
      (Utilities|FlowControl|DoOnce false) ; enters at Reset
    )))

(event Custom|PickRandomSpawnPoint
  (bind (_randomzone _zoneindex) (CallFunction|PickRandomZone))
  (bind (_randompoint _pointindex) (CallFunction|PickRandomPoint))
  (if (< (Variables|CurrentWave|GetCurrentWaveSpawnedEnemies) (Variables|/Game/Gameplay/AI/Spawn/Waves/PDA_WaveData.PDA_WaveData_C|GetAmount (Variables|CurrentWave|GetCurrentWave)))
    (if (< (Variables|Default|GetEnemyCount) (Variables|CurrentWave|GetCurrentWaveMaxCap))
      (CallFunction|ResetDefferedSpawnTimer)
      (if (or (Variables|CurrentWave|GetCurretWaveHasZones) (Variables|CurrentWave|GetCurretWaveHasPoints))
        (if (> (Math|Random|RandomFloat) 0.5)
          (Utilities|FlowControl|DoOnce false :!label _label
            (:Completed
              (if (Variables|CurrentWave|GetCurretWaveHasZones)
                (CallFunction|SpawnfromZone _randomzone _zoneindex)
                (else
                  (Utilities|FlowControl|DoOnce false :!label _label_2
                    (:Completed
                      (if (Variables|CurrentWave|GetCurretWaveHasPoints)
                        (CallFunction|SpawnfromPoint _randompoint _pointindex)
                        (else
                          (goto _label)))))))))
          (else
            (goto _label_2)))
        (CallFunction|ResetGatesforSpawn)
        (else
          (Utilities|Debugging|RaiseScriptError "No Boxes/Zones in current Wave")))
      (elif (not (Utilities|Time|IsValidTimerHandle (Variables|Deffered|GetSpawnDefferedTimer)))
        (bind _returnvalue (Utilities|Time|SetTimerbyEvent (EventDispatchers|CreateEvent :!event Custom|PickRandomSpawnPoint) 2.0 true true))
        (Variables|Deffered|SetSpawnDefferedTimer _returnvalue)))
    (else
      (Default|CallNoMoreEnemiestoSpawninThisWave)
      (CallFunction|SetupNewWave false false))))

(event Custom|SpawnFromZone
  (params (ZoneData :type S%20Trigger%20Box%20Structure) (ZoneIndex :type Integer))
  (bind _triggerbox (Utilities|Struct|BreakS_TriggerBox ZoneData))
  (bind _object (Utilities|AsyncLoadAsset _triggerbox)
    (:Completed
      (Utilities|IsValid _object
        (:Is%20Valid
          (bind _spawnedenemy (CallFunction|SpawnEnemy (Utilities|ResolveSoftReference _triggerbox) 0 (Variables|/Game/Gameplay/AI/Spawn/Waves/PDA_WaveData.PDA_WaveData_C|GetAutoAggro (Variables|CurrentWave|GetCurrentWave)) 0.0))
          (Utilities|IsValid _spawnedenemy
            (:Is%20Valid
              (Game|BindEventtoOnDestroyed _spawnedenemy (EventDispatchers|CreateEvent :!event Custom|OnEnemyDestroyed)))
            (:Is%20Not%20Valid
              _))
          (switch Utilities|FlowControl|Switch|SwitchonE_WaveSpawnType (Variables|/Game/Gameplay/AI/Spawn/Waves/PDA_WaveData.PDA_WaveData_C|GetSpawnType (Variables|CurrentWave|GetCurrentWave))
            (:NewEnumerator0
              (Utilities|FlowControl|Delay (/ 1.0 (Variables|/Game/Gameplay/AI/Spawn/Waves/PDA_WaveData.PDA_WaveData_C|GetEnemiesPerSecond (Variables|CurrentWave|GetCurrentWave)))))
            (:NewEnumerator1
              (Utilities|FlowControl|DelayUntilNextTick)))
          (CallFunction|PickRandomSpawnPoint))
        (:Is%20Not%20Valid
          (Utilities|Debugging|RaiseScriptError "Invalid TriggerBox"))))))

(event Custom|SpawnFromPoint
  (params (SpawnPointData :type S%20Spawn%20Point%20Structure) (SpawnPointIndex :type Integer))
  (bind (_spawnpoint _priority _spawndispersion) (Utilities|Struct|BreakS_SpawnPoint SpawnPointData))
  (bind _object (Utilities|AsyncLoadAsset _spawnpoint)
    (:Completed
      (Utilities|IsValid _object
        (:Is%20Valid
          (bind _spawnedenemy (CallFunction|SpawnEnemy 0 (Utilities|ResolveSoftReference _spawnpoint) (Variables|/Game/Gameplay/AI/Spawn/Waves/PDA_WaveData.PDA_WaveData_C|GetAutoAggro (Variables|CurrentWave|GetCurrentWave)) _spawndispersion))
          (Utilities|IsValid _spawnedenemy
            (:Is%20Valid
              (Game|BindEventtoOnDestroyed _spawnedenemy (EventDispatchers|CreateEvent :!event Custom|OnEnemyDestroyed))
              (EventDispatchers|BindEventtoEnemyDied _spawnedenemy (EventDispatchers|CreateEvent :!event OnEnemyDie)))
            (:Is%20Not%20Valid
              _))
          (switch Utilities|FlowControl|Switch|SwitchonE_WaveSpawnType (Variables|/Game/Gameplay/AI/Spawn/Waves/PDA_WaveData.PDA_WaveData_C|GetSpawnType (Variables|CurrentWave|GetCurrentWave))
            (:NewEnumerator0
              (Utilities|FlowControl|Delay (/ 1.0 (Variables|/Game/Gameplay/AI/Spawn/Waves/PDA_WaveData.PDA_WaveData_C|GetEnemiesPerSecond (Variables|CurrentWave|GetCurrentWave)))))
            (:NewEnumerator1
              (Utilities|FlowControl|DelayUntilNextTick)))
          (CallFunction|PickRandomSpawnPoint))
        (:Is%20Not%20Valid
          (Utilities|Debugging|RaiseScriptError "Invalid Spawner"))))))

(event Custom|DefferedStartWave
  (if (<= (Variables|Default|GetEnemyCount) 0)
    (Variables|Deffered|SetForcedStart true)
    (Utilities|FlowControl|Sequence
      (:then_0
        (CallFunction|ResetDefferedStartWave)
        (CallFunction|ExtractPriorities)
        (CallFunction|DoesWaveHasZonesorBoxes)
        (Spawners|CloseSpawnPoints)
        (Utilities|FlowControl|Sequence
          (:then_0
            (CallFunction|EnrageAliveEnemies)
            (Audio|PlaySound2D (Variables|Default|GetBeginWaveCue) 0.5 1.0 11.0 0 0)
            (Utilities|FlowControl|Delay 2.0)
            (Spawners|OpenSpawnPoints)
            (Development|PrintString (Utilities|String|Append "NEW WAVE : " (Utilities|String|ToString(Integer) (Variables|Default|GetWaveIndex))) true true "(R=1.000000,G=0.000000,B=0.022609,A=1.000000)" 1e+01))
          (:then_1
            (Utilities|FlowControl|Delay 4.0)
            (CallFunction|PickRandomSpawnPoint))))
      (:then_1
        (Default|LerptoNewPercent (Variables|Default|GetHUD) 1.0 0.025)))))

(event EventBeginPlay
  (bind _continue (CallFunction|HandleGameMode))
  (if (and _continue (Variables|Default|GetAutoStart))
    (Utilities|FlowControl|DelayUntilNextTick)
    (bind _asbp_fps_character (Utilities|Casting|CastToBP_FPS_Character (Game|Player|GetPlayerPawn 0))
      (:then
        (Variables|Default|SetHUD (Variables|/Game/Gameplay/Player/BP_FPS_Character.BP_FPS_Character_C|GetWBP_HUD _asbp_fps_character)))
      (:CastFailed
        (Development|PrintString "failed cast")))
    (bind _outactors (Actor|GetAllActorsOfClass "/Game/Gameplay/AI/Spawn/BP_SpawnPoint.BP_SpawnPoint_C"))
    (Variables|Default|SetSpawnPoints _outactors)
    (Spawners|CloseSpawnPoints)
    (CallFunction|SetupNewWave true false)))

(event Collision|EventActorBeginOverlap
  (params (OtherActor :type Actor%20Object%20Reference)))

(event EventTick
  (params (DeltaSeconds :type Float%20%28single-precision%29)))

(fn ConstructionScript
  (Rendering|Components|TextRender|SetText (Variables|Default|GetTextRender) (Utilities|Text|ToText(String) (Utilities|GetDisplayName self))))

(fn SpawnEnemy
  (params (TriggerBox :type Trigger%20Box%20Object%20Reference) (SpawnPoint :type BP%20Spawn%20Point%20Object%20Reference) (AutoAggro :type Boolean) (SpawnDispersion :type Float%20%28double-precision%29))
  (bind (_origin _boxextent) (Collision|GetActorBounds TriggerBox false false))
  (bind _returnvalue (Math|Random|RandomFloatinRange 0.0 SpawnDispersion))
  (bind _freeenemies (Variables|Pool|GetFreeEnemies))
  (bind _freeenemies_2 (Variables|Pool|GetFreeEnemies))
  (LocalVariables|SetLAutoAggro AutoAggro)
  (Utilities|IsValid TriggerBox
    (:Is%20Valid
      (bind _output_get (LocalVariables|SetLRandomPoint (Math|Random|RandomPointinBoundingBox _origin _boxextent)))
      (bind (_outhit _returnvalue_2) (Collision|LineTraceByChannel _output_get (+ _output_get (* (Math|Vector|GetUpVector "0, 0, 0") -1.0 (Math|Vector|VectorLength _boxextent))) "TraceTypeQuery1" false 0 "ForDuration"))
      (if _returnvalue_2
        (LocalVariables|SetLSpawnPoint (.Location (Collision|BreakHitResult _outhit)))
        (else
          (return 0))))
    (:Is%20Not%20Valid
      (Utilities|IsValid SpawnPoint
        (:Is%20Valid
          (bind _output_get_2 (LocalVariables|SetLRandomPoint (+ (Transformation|GetActorLocation SpawnPoint) (* (Math|Random|RandomUnitVector) (Math|Vector|MakeVector _returnvalue _returnvalue 0.0)))))
          (bind (_outhit_2 _returnvalue_3) (Collision|LineTraceByChannel _output_get_2 (+ _output_get_2 (* (Transformation|GetActorUpVector SpawnPoint) -1.0 (Math|Float|MakeLiteralFloat 5e+02))) "TraceTypeQuery1" false 0 "None"))
          (if _returnvalue_3
            (LocalVariables|SetLSpawnPoint (+ (.Location (Collision|BreakHitResult _outhit_2)) "0.000000,0.000000,150.000000"))
            (else
              (return 0))))
        (:Is%20Not%20Valid
          (return 0)))))
  (if (> (Utilities|Array|Length _freeenemies_2) 0)
    (bind _output_get_3 (LocalVariables|SetEnemyRef (Utilities|ResolveSoftReference (Utilities|Array|Get(acopy) (Variables|Pool|GetEnemies) (Utilities|Array|Get(acopy) _freeenemies_2 (Utilities|Array|LastIndex _freeenemies_2))))))
    (Utilities|IsValid _output_get_3
      (:Is%20Valid
        (Default|PreparetoHold _output_get_3)
        (Default|ResettoInitialState _output_get_3)
        (Default|PreparetoSpawn _output_get_3)
        (Transformation|SetActorLocation _output_get_3 (LocalVariables|GetLSpawnPoint) false false)
        (Utilities|Array|RemoveIndex _freeenemies (Utilities|Array|LastIndex _freeenemies))
        (LocalVariables|SetEnemyId (Variables|/Game/Gameplay/AI/Pooling/BPC_PooledActor.BPC_PooledActor_C|GetPoolId (Variables|/Game/Gameplay/AI/BP_Enemy.BP_Enemy_C|GetBPC_PooledActor (LocalVariables|GetEnemyRef))))
        (Utilities|Array|RemoveItem _freeenemies (Utilities|Array|FindItem _freeenemies (Variables|/Game/Gameplay/AI/Pooling/BPC_PooledActor.BPC_PooledActor_C|GetPoolId (Variables|/Game/Gameplay/AI/BP_Enemy.BP_Enemy_C|GetBPC_PooledActor (LocalVariables|GetEnemyRef)))))
        (Utilities|IsValid (LocalVariables|GetEnemyRef)
          (:Is%20Valid
            (Math|Integer|IncrementInt (Variables|CurrentWave|GetCurrentWaveSpawnedEnemies)
              (:%20%20
                (bind _result (Math|Integer|IncrementInt (Variables|Default|GetEnemyCount))
                  (:%20%20
                    (Default|UpdateEnemyAmount (Variables|Default|GetHUD) _result)
                    (Utilities|Array|Add (Variables|Rage|GetAliveEnemyIds) (LocalVariables|GetEnemyId))
                    (return (LocalVariables|GetEnemyRef)))))))
          (:Is%20Not%20Valid
            (return 0))))
      (:Is%20Not%20Valid
        (Utilities|Debugging|RaiseScriptError "GOTCHA, invalid ref")))
    (else
      (return 0))))

(fn ExtractPriorities
  (bind _currentwave (Variables|CurrentWave|GetCurrentWave))
  (Utilities|Array|Clear (Variables|CurrentWave|GetCurrentWaveZonePriority))
  (Utilities|Array|Clear (Variables|CurrentWave|GetCurrentWaveSpawnersPriority))
  (for _array_element (Variables|/Game/Gameplay/AI/Spawn/Waves/PDA_WaveData.PDA_WaveData_C|GetSpawners _currentwave)
    (Utilities|Array|Add (Variables|CurrentWave|GetCurrentWaveSpawnersPriority) (.Priority (Utilities|Struct|BreakS_SpawnPoint _array_element))))
  (for _array_element_2 (Variables|/Game/Gameplay/AI/Spawn/Waves/PDA_WaveData.PDA_WaveData_C|GetBoxes _currentwave)
    (Utilities|Array|Add (Variables|CurrentWave|GetCurrentWaveZonePriority) (.Priority (Utilities|Struct|BreakS_TriggerBox _array_element_2))))
  (return))

(fn DoesWaveHasZonesorBoxes
  (Variables|CurrentWave|SetCurretWaveHasPoints (> (Utilities|Array|Length (Variables|/Game/Gameplay/AI/Spawn/Waves/PDA_WaveData.PDA_WaveData_C|GetSpawners (Variables|CurrentWave|GetCurrentWave))) 0))
  (Variables|CurrentWave|SetCurretWaveHasZones (> (Utilities|Array|Length (Variables|/Game/Gameplay/AI/Spawn/Waves/PDA_WaveData.PDA_WaveData_C|GetBoxes (Variables|CurrentWave|GetCurrentWave))) 0))
  (return))

(fn PickRandomZone
  (bind _currentwave (Variables|CurrentWave|GetCurrentWave))
  (bind _boxes (Variables|/Game/Gameplay/AI/Spawn/Waves/PDA_WaveData.PDA_WaveData_C|GetBoxes _currentwave))
  (bind (_outitem _outindex) (Utilities|Array|Random _boxes))
  (return _outitem _outindex))

(fn PickRandomPoint
  (bind _currentwave (Variables|CurrentWave|GetCurrentWave))
  (bind _spawners (Variables|/Game/Gameplay/AI/Spawn/Waves/PDA_WaveData.PDA_WaveData_C|GetSpawners _currentwave))
  (bind (_outitem _outindex) (Utilities|Array|Random _spawners))
  (return _outitem _outindex))

(fn PreSpawnEnemy
  (bind _returnvalue (Game|SpawnActorfromClass "/Game/Gameplay/AI/BP_Enemy.BP_Enemy_C" (Math|Transform|MakeTransform "0, 0, 0" "0, 0, 0" "1.000000,1.000000,1.000000") "Undefined" "MultiplyWithRoot" 0 true "NewEnumerator0" 0))
  (Default|PreparetoHold _returnvalue)
  (bind _returnvalue_2 (Utilities|Array|Add (Variables|Pool|GetEnemies) (Utilities|ResolveSoftReference _returnvalue)))
  (bind _output_get (Variables|/Game/Gameplay/AI/Pooling/BPC_PooledActor.BPC_PooledActor_C|SetPoolId (Variables|/Game/Gameplay/AI/BP_Enemy.BP_Enemy_C|GetBPC_PooledActor _returnvalue) _returnvalue_2))
  (Utilities|Array|Add (Variables|Pool|GetFreeEnemies) _output_get))

(fn OnEnemyDie
  (params (ActorRef :type BP%20Enemy%20Object%20Reference) (Reset? :type Boolean))
  (bind _bpc_pooledactor (Variables|/Game/Gameplay/AI/BP_Enemy.BP_Enemy_C|GetBPC_PooledActor ActorRef))
  (bind _hud (Variables|Default|GetHUD))
  (bind _aliveenemyids (Variables|Rage|GetAliveEnemyIds))
  (bind _poolid (Variables|/Game/Gameplay/AI/Pooling/BPC_PooledActor.BPC_PooledActor_C|GetPoolId _bpc_pooledactor))
  (bind _returnvalue (Utilities|Array|FindItem _aliveenemyids _poolid))
  (if (Variables|/Game/Gameplay/AI/BP_Enemy.BP_Enemy_C|GetCalledDeathAlready ActorRef)
    _
    (else
      (bind _result (Math|Integer|DecrementInt (Variables|Default|GetEnemyCount))
        (:%20%20
          (Default|UpdateEnemyAmount _hud _result)
          (Default|IncrementComboKill _hud)))))
  (if (and Reset? (Variables|/Game/Gameplay/AI/Pooling/BPC_PooledActor.BPC_PooledActor_C|GetInUse (Variables|/Game/Gameplay/AI/BP_Enemy.BP_Enemy_C|GetBPC_PooledActor ActorRef)))
    (Transformation|SetActorLocation ActorRef "0, 0, 0" false false)
    (if (== (Utilities|Array|FindItem (Variables|Pool|GetFreeEnemies) (Variables|/Game/Gameplay/AI/Pooling/BPC_PooledActor.BPC_PooledActor_C|GetPoolId (Variables|/Game/Gameplay/AI/BP_Enemy.BP_Enemy_C|GetBPC_PooledActor ActorRef))) -1)
      (if (Utilities|Array|IsValidIndex _aliveenemyids _returnvalue)
        (Utilities|Array|RemoveItem (Variables|Rage|GetAliveEnemyIds) _returnvalue))
      (Default|ResettoInitialState ActorRef)
      (Default|PreparetoHold ActorRef)
      (Utilities|Array|Add (Variables|Pool|GetFreeEnemies) (Variables|/Game/Gameplay/AI/Pooling/BPC_PooledActor.BPC_PooledActor_C|GetPoolId (Variables|/Game/Gameplay/AI/BP_Enemy.BP_Enemy_C|GetBPC_PooledActor ActorRef)))
      (CallFunction|CheckEndGame)
      (else
        (Utilities|Debugging|RaiseScriptError "DUPILCATE")
        (Development|PrintString "BIG FUCK UP")))
    (else
      (CallFunction|CheckEndGame))))

(fn EnrageAliveEnemies
  (for _array_element (Variables|Rage|GetAliveEnemyIds)
    (bind _returnvalue (Utilities|LoadAssetBlocking (Utilities|Array|Get(acopy) (Variables|Pool|GetEnemies) _array_element)))
    (bind _asbp_enemy (Utilities|Casting|CastToBP_Enemy _returnvalue))
    (Default|ApplyRage _asbp_enemy)))

(fn CheckEndGame
  (bind _waves (Variables|Default|GetWaves))
  (bind _waveindex (Variables|Default|GetWaveIndex))
  (bind _returnvalue (Utilities|Array|Length _waves))
  (if (and (or (== _returnvalue _waveindex) (== _returnvalue (+ _waveindex 1))) (== (Variables|Default|GetEnemyCount) 0))
    (if (== (Variables|CurrentWave|GetCurrentWaveSpawnedEnemies) (Variables|/Game/Gameplay/AI/Spawn/Waves/PDA_WaveData.PDA_WaveData_C|GetAmount (Variables|CurrentWave|GetCurrentWave)))
      (Default|CallEndOfGame)
      (Development|PrintString "GameEnd")
      (Utilities|Debugging|RaiseScriptError "END OF GAME"))))

(fn OpenSpawnPoints
  (for _array_element (Variables|/Game/Gameplay/AI/Spawn/Waves/PDA_WaveData.PDA_WaveData_C|GetSpawners (Variables|CurrentWave|GetCurrentWave))
    (Utilities|LoadAssetBlocking (.SpawnPoint (Utilities|Struct|BreakS_SpawnPoint _array_element)))
    (Default|OpenSpawner (Utilities|ResolveSoftReference (.SpawnPoint (Utilities|Struct|BreakS_SpawnPoint _array_element))))))

(fn CloseSpawnPoints
  (for _array_element (Variables|Default|GetSpawnPoints)
    (Utilities|IsValid _array_element
      (:Is%20Valid
        (Default|CloseSpawner _array_element)))))

(fn HandleGameMode
  (bind _returnvalue (Game|GetGameMode))
  (Utilities|Casting|CastToBP_FPS_GameModeMain _returnvalue
    (:then
      (return true))
    (:CastFailed
      (bind _asbp_gm_front (Utilities|Casting|CastToBP_GM_Front _returnvalue)
        (:then
          (EventDispatchers|BindEventtoStartGame _asbp_gm_front (EventDispatchers|CreateEvent :!event Custom|MenuStart))
          (return false))
        (:CastFailed
          (return true))))))