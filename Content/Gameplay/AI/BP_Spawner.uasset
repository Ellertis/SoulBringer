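; BP_Spawner is an actor that spawns BP_Enemy pawns at its own location with a random yaw between -90 and 90 degrees.
; SpawnSmart spawns an enemy and leaves its AI running.
; SpawnBrainDead spawns one, then gets its AIC_Enemy controller and stops the StateTreeAI logic, leaving it inert.
; Nothing in the blueprint calls either event, so spawning is triggered externally.
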(event Custom|SpawnSmart
  (Game|SpawnActorfromClass "/Game/Gameplay/AI/BP_Enemy.BP_Enemy_C" (Math|Transform|MakeTransform (Transformation|GetActorLocation) (Math|Rotator|MakeRotator 0.0 0.0 (Math|Random|RandomFloatinRange -9e+01 9e+01)) "1.000000,1.000000,1.000000") "Undefined" "MultiplyWithRoot" 0 0))

(event Custom|SpawnBrainDead
  (bind _returnvalue (Game|SpawnActorfromClass "/Game/Gameplay/AI/BP_Enemy.BP_Enemy_C" (Math|Transform|MakeTransform (Transformation|GetActorLocation) (Math|Rotator|MakeRotator 0.0 0.0 (Math|Random|RandomFloatinRange -9e+01 9e+01)) "1.000000,1.000000,1.000000") "Undefined" "MultiplyWithRoot" 0 0))
  (bind _asaic_enemy (Utilities|Casting|CastToAIC_Enemy (AI|GetAIController _returnvalue)))
  (AI|Logic|StopLogic (Variables|/Game/Gameplay/AI/AIC_Enemy.AIC_Enemy_C|GetStateTreeAI _asaic_enemy) ""))

(event EventBeginPlay)

(event Collision|EventActorBeginOverlap
  (params (OtherActor :type Actor%20Object%20Reference)))

(event EventTick
  (params (DeltaSeconds :type Float%20%28single-precision%29)))

(fn ConstructionScript)