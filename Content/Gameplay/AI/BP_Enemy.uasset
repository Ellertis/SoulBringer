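; Enemy character that can be pulled, held and thrown as a physics object, sticking to what it hits and carrying a parasite effect.
; Pulling stops its StateTree AI and simulates a sphere proxy or ragdoll, with a looping timer keeping the capsule on it.
; Once thrown, a valid hit freezes and attaches it to the target, optionally starting a delayed parasite explosion.
; Also handles montage attacks, HP damage with ragdoll death, and destruction when the parasite explodes.
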(event Custom|Attack
  (Animation|Montage|PlayMontage (Variables|Character|GetMesh) "/Game/Variant_Shooter/Anims/FP_Rifle_Shoot_Montage.FP_Rifle_Shoot_Montage"
    (:OnCompleted
      _)
    (:OnInterrupted
      _))
  (Default|CallAttackFinished))

(event Custom|SnapCapsuleToSphere
  (Transformation|SetWorldLocation (Variables|Collision|GetCapsuleComponent) (Transformation|GetWorldLocation (Variables|Default|GetSphere)) false false))

(event Custom|SnapCapsuleToSkeletalMesh
  (Transformation|SetWorldLocation (Variables|Collision|GetCapsuleComponent) (Transformation|GetSocketLocation (Variables|Character|GetMesh) "pelvis") false false))

(event Custom|Die
  (bind _mesh (Variables|Character|GetMesh))
  (Components|Activation|Deactivate (Variables|Character|GetCharacterMovement))
  (Collision|SetCollisionProfileName _mesh "Ragdoll" false :!class /Script/Engine.PrimitiveComponent)
  (Physics|SetSimulatePhysics _mesh true)
  (Collision|SetCollisionEnabled (Variables|Collision|GetCapsuleComponent) "NoCollision"))

(event Custom|ExplosionProc
  (Rendering|SetVisibility (Variables|Default|GetGC_Liquide) true false)
  (Audio|Components|Audio|Play (Variables|Default|GetGC_Liquide))
  (Actor|DestroyActor))

(event EventBeginPlay
  (Variables|/Game/Gameplay/Parasite/BPC_Parasite.BPC_Parasite_C|SetMeshToAffect (Variables|Default|GetBPC_Parasite) (Variables|Default|GetSphere))
  (EventDispatchers|BindEventtoExplosionTriggered (Variables|Default|GetBPC_Parasite) (EventDispatchers|CreateEvent :!event Custom|ExplosionProc)))

(event Collision|EventActorBeginOverlap
  (params (OtherActor :type Actor%20Object%20Reference)))

(event Collision|EventHit
  (params (MyComp :type Primitive%20Component%20Object%20Reference) (Other :type Actor%20Object%20Reference) (OtherComp :type Primitive%20Component%20Object%20Reference) (bSelfMoved :type Boolean) (HitLocation :type Vector :default "0, 0, 0") (HitNormal :type Vector :default "0, 0, 0") (NormalImpulse :type Vector :default "0, 0, 0") (Hit :type Hit%20Result%20Structure%20%28by%20ref%29))
  (bind (_bblockinghit _binitialoverlap _time _distance _location _impactpoint _normal _impactnormal _physmat _hitactor _hitcomponent) (Collision|BreakHitResult Hit))
  (bind _sphere (Variables|Default|GetSphere))
  (bind _mesh (Variables|Character|GetMesh))
  (bind _bpc_parasite (Variables|Default|GetBPC_Parasite))
  (switch Utilities|FlowControl|Switch|SwitchonGrabState (Variables|Default|GetGrabState)
    (:NewEnumerator2
      (Development|PrintString "THROWN" true false "(R=0.000000,G=0.660000,B=1.000000,A=1.000000)" 0.1)
      (if (Math|Boolean|ANDBoolean (!= _hitactor self) (!= _hitcomponent (Variables|Character|GetMesh)) (not (Actor|ActorHasTag _hitactor "Projectile")))
        (Development|PrintString "GOT HIM")
        (Variables|Default|SetGrabState "NewEnumerator3")
        (if (Variables|Default|GetKeepRagdoll)
          (Utilities|Time|ClearandInvalidateTimerbyHandle (Variables|Default|GetRagdollTimer))
          (Class|PrimitiveComponent|SetAllPhysicsLinearVelocity _mesh "0, 0, 0" false)
          (Class|PrimitiveComponent|SetAllPhysicsAngularVelocityinDegrees _mesh (Math|Vector|MakeVector 0.0 0.0 0.0) false)
          (Class|PrimitiveComponent|PutRigidBodytoSleep _mesh "None")
          (Components|Tick|SetComponentTickEnabled _mesh false)
          (Physics|SetSimulatePhysics _mesh false)
          (Physics|SetEnableGravity _mesh false)
          (Collision|SetCollisionResponsetoChannel _mesh "ECC_Pawn" "ECR_Ignore")
          (Transformation|AttachComponentToComponent (Variables|Character|GetMesh) (Variables|Collision|GetCapsuleComponent) "None" "KeepWorld" "KeepWorld" "KeepWorld" false)
          (Transformation|AttachActorToActor _hitactor "None" "KeepWorld" "KeepWorld" "KeepWorld" false)
          (else
            (Class|PrimitiveComponent|SetAllPhysicsLinearVelocity _sphere "0, 0, 0" false)
            (Class|PrimitiveComponent|SetAllPhysicsAngularVelocityinDegrees _sphere (Math|Vector|MakeVector 0.0 0.0 0.0) false)
            (Physics|SetSimulatePhysics _sphere false)
            (Physics|SetEnableGravity _sphere false)
            (Collision|SetCollisionResponsetoChannel _sphere "ECC_Pawn" "ECR_Ignore")
            (Collision|SetCollisionResponsetoChannel _sphere "ECC_GameTraceChannel1" "ECR_Ignore")
            (Transformation|SetWorldLocation (Variables|Collision|GetCapsuleComponent) (Transformation|GetWorldLocation (Variables|Default|GetSphere)) false false)
            (Transformation|AttachComponentToComponent (Variables|Default|GetSphere) (Variables|Collision|GetCapsuleComponent) "None" "KeepWorld" "KeepWorld" "KeepWorld" false)
            (Transformation|AttachActorToActor _hitactor "None" "KeepWorld" "KeepWorld" "KeepWorld" false)
            (Utilities|Time|ClearandInvalidateTimerbyHandle (Variables|Default|GetRagdollTimer))))
        (if (Variables|/Game/Gameplay/Parasite/PDA_ParasiteData.PDA_ParasiteData_C|GetDelayedExplosionOnContact (Variables|/Game/Gameplay/Parasite/BPC_Parasite.BPC_Parasite_C|GetEntityParasiteData _bpc_parasite))
          (Default|DelayedExplosion _bpc_parasite))))))

(event Game|Damage|EventAnyDamage
  (params (Damage :type Float%20%28single-precision%29) (DamageType :type Damage%20Type%20Object%20Reference) (InstigatedBy :type Controller%20Object%20Reference) (DamageCauser :type Actor%20Object%20Reference))
  (if (> (Variables|Default|GetHP) 0.0)
    (bind _output_get (Variables|Default|SetHP (- (Variables|Default|GetHP) Damage)))
    (if (<= _output_get 0.0)
      (CallFunction|Die))))

(event EventOnPullObject
  (bind _sphere (Variables|Default|GetSphere))
  (bind _capsulecomponent (Variables|Collision|GetCapsuleComponent))
  (bind _bpc_parasite (Variables|Default|GetBPC_Parasite))
  (bind _capsulecomponent_2 (Variables|Collision|GetCapsuleComponent))
  (bind _mesh (Variables|Character|GetMesh))
  (Components|Activation|Deactivate (Variables|Character|GetCharacterMovement))
  (bind _asaic_enemy (Utilities|Casting|CastToAIC_Enemy (AI|GetAIController self))
    (:then
      (AI|Logic|StopLogic (Variables|/Game/Gameplay/AI/AIC_Enemy.AIC_Enemy_C|GetStateTreeAI _asaic_enemy) ""))
    (:CastFailed
      _))
  (if (Variables|Default|GetKeepRagdoll)
    (Collision|SetCollisionProfileName _mesh "Ragdoll" false :!class /Script/Engine.PrimitiveComponent)
    (Physics|SetSimulatePhysics _mesh true)
    (Collision|SetCollisionResponsetoChannel _mesh "ECC_Pawn" "ECR_Block")
    (Collision|SetCollisionEnabled _capsulecomponent "NoCollision")
    (Physics|SetEnableGravity _capsulecomponent false)
    (bind _returnvalue (Utilities|Time|SetTimerbyEvent (delegate Custom|SnapCapsuleToSkeletalMesh) 0.001 true))
    (Variables|Default|SetRagdollTimer _returnvalue)
    (else
      (Collision|SetCollisionProfileName _sphere "Ragdoll" false :!class /Script/Engine.PrimitiveComponent)
      (Collision|SetCollisionResponsetoChannel _sphere "ECC_Pawn" "ECR_Block")
      (Physics|SetSimulatePhysics _sphere true)
      (Physics|SetEnableGravity (Variables|Default|GetSphere) true)
      (Collision|SetCollisionEnabled _capsulecomponent_2 "NoCollision")
      (Physics|SetEnableGravity _capsulecomponent_2 false)
      (Collision|SetCollisionEnabled (Variables|Character|GetMesh) "NoCollision")
      (bind _returnvalue_2 (Utilities|Time|SetTimerbyEvent (delegate Custom|SnapCapsuleToSphere) 0.001 true))
      (Variables|Default|SetRagdollTimer _returnvalue_2)))
  (Variables|Default|SetGrabState "NewEnumerator1")
  (Rendering|SetVisibility (Variables|Character|GetMesh) false false)
  (Rendering|SetVisibility (Variables|Default|GetSphere) true false)
  (Default|ProcParasite _bpc_parasite)
  (if (Variables|/Game/Gameplay/Parasite/PDA_ParasiteData.PDA_ParasiteData_C|GetProcInHand (Variables|/Game/Gameplay/Parasite/BPC_Parasite.BPC_Parasite_C|GetEntityParasiteData _bpc_parasite))
    (Default|StartProcTimer _bpc_parasite)))

(event EventOnHitObject
  (params (HitResult :type Hit%20Result%20Structure))
  (if (Utilities|Enum|NotEqual(Enum) (Variables|Default|GetGrabState) "NewEnumerator1")
    (Default|TrytoProc (Variables|Default|GetBPC_Parasite))))

(event EventOnPushObject
  (bind _bpc_parasite (Variables|Default|GetBPC_Parasite))
  (Variables|Default|SetGrabState "NewEnumerator2")
  (if (Variables|/Game/Gameplay/Parasite/PDA_ParasiteData.PDA_ParasiteData_C|GetProcInHand (Variables|/Game/Gameplay/Parasite/BPC_Parasite.BPC_Parasite_C|GetEntityParasiteData _bpc_parasite))
    (Default|StopProcTimer _bpc_parasite)))

(fn ConstructionScript)

(fn GetGrabbableComponent
  (return (Variables|Default|GetSphere)))