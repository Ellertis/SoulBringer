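; Actor component that infects its owner with a parasite charge and makes it explode when full, tuned by EntityParasiteData.
; Procs from bullet counts or increments, optionally on a looping timer, raise ParasiteLevel and drive a dynamic overlay material.
; At maximum it explodes after a delay, or flags grabbed enemies to die on contact.
; Explosions push physics objects and players by charge, destroy nearby non-grabbed enemies and spawn charge-scaled Niagara effects.
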(event Custom|TryToProc
  (if (>= (Variables|Data|GetParasiteLevel) (Variables|/Game/Gameplay/Parasite/PDA_ParasiteData.PDA_ParasiteData_C|GetParasiteMin (Variables|Data|GetEntityParasiteData)))
    (CallFunction|ProcParasite)))

(event Custom|ProcParasite
  (bind _entityparasitedata (Variables|Data|GetEntityParasiteData))
  (bind _entityparasitedata_2 (Variables|Data|GetEntityParasiteData))
  (Utilities|IsValid (Variables|Functional|GetParasiteMID)
    (:Is%20Valid
      _)
    (:Is%20Not%20Valid
      (bind _returnvalue (Rendering|Material|CreateDynamicMaterialInstance (Variables|/Game/Gameplay/Parasite/PDA_ParasiteData.PDA_ParasiteData_C|GetParasiteMaterial (Variables|Data|GetEntityParasiteData)) "None" "None" :!class /Script/Engine.KismetMaterialLibrary))
      (bind _output_get (Variables|Functional|SetParasiteMID _returnvalue))
      (Rendering|Material|SetOverlayMaterial (Variables|Functional|GetMeshToAffect) _output_get :!class /Script/Engine.MeshComponent)))
  (if (Variables|/Game/Gameplay/Parasite/PDA_ParasiteData.PDA_ParasiteData_C|GetUseBulletCountInsteadOfParasiteValue (Variables|Data|GetEntityParasiteData))
    (Math|Integer|IncrementInt (Variables|Data|GetBulletsTaken)
      (:%20%20
        (CallFunction|ConvertBulletstoParasite)
        (CallFunction|UpdateParasiteMaterial (>= (Variables|Data|GetParasiteLevel) (Variables|/Game/Gameplay/Parasite/PDA_ParasiteData.PDA_ParasiteData_C|GetParasiteMax (Variables|Data|GetEntityParasiteData))))
        (Audio|PlaySound2D "/Game/Gameplay/SoundPlaceHolder/PHS_LC_To_RcPlaceHolder_Cue.PHS_LC_To_RcPlaceHolder_Cue" 1.0 1.0 0.0 0 0)
        (if (>= (Variables|Data|GetBulletsTaken) (+ (Variables|/Game/Gameplay/Parasite/PDA_ParasiteData.PDA_ParasiteData_C|GetBulletsToExplode _entityparasitedata_2) 1))
          (bind _asbp_enemy (Utilities|Casting|CastToBP_Enemy (Components|GetOwner))
            (:then
              (if (Utilities|Enum|Equal(Enum) (Variables|/Game/Gameplay/AI/BP_Enemy.BP_Enemy_C|GetGrabState _asbp_enemy) "NewEnumerator2")
                (if (Variables|/Game/Gameplay/Parasite/PDA_ParasiteData.PDA_ParasiteData_C|GetExplodeInAir (Variables|Data|GetEntityParasiteData))
                  (Utilities|FlowControl|Delay (Variables|/Game/Gameplay/Parasite/PDA_ParasiteData.PDA_ParasiteData_C|GetExplosionDelay _entityparasitedata_2) :!label _label)
                  (CallFunction|DelayedExplosion)
                  (else
                    (Variables|Functional|SetShouldDieOnContact true)))
                (else
                  (goto _label))))
            (:CastFailed
              (goto _label))))))
    (else
      (bind _output_get_2 (Variables|Data|SetParasiteLevel (Math|Float|Clamp(Float) (+ (Variables|Data|GetParasiteLevel) (Variables|/Game/Gameplay/Parasite/PDA_ParasiteData.PDA_ParasiteData_C|GetParasiteProcIncrease _entityparasitedata)) (Variables|/Game/Gameplay/Parasite/PDA_ParasiteData.PDA_ParasiteData_C|GetParasiteMin _entityparasitedata) (Variables|/Game/Gameplay/Parasite/PDA_ParasiteData.PDA_ParasiteData_C|GetParasiteMax _entityparasitedata))))
      (CallFunction|UpdateParasiteMaterial (>= _output_get_2 (Variables|/Game/Gameplay/Parasite/PDA_ParasiteData.PDA_ParasiteData_C|GetParasiteMax (Variables|Data|GetEntityParasiteData))))
      (if (>= _output_get_2 (Variables|/Game/Gameplay/Parasite/PDA_ParasiteData.PDA_ParasiteData_C|GetParasiteMax (Variables|Data|GetEntityParasiteData)))
        (goto _label)))))

(event Custom|Explosion
  (bind _entityparasitedata (Variables|Data|GetEntityParasiteData))
  (bind _entityparasitedata_2 (Variables|Data|GetEntityParasiteData))
  (bind _parasitelevel (Variables|Data|GetParasiteLevel))
  (bind _parasitemax (Variables|/Game/Gameplay/Parasite/PDA_ParasiteData.PDA_ParasiteData_C|GetParasiteMax _entityparasitedata_2))
  (bind _parasitemin (Variables|/Game/Gameplay/Parasite/PDA_ParasiteData.PDA_ParasiteData_C|GetParasiteMin _entityparasitedata_2))
  (bind _explosionniagarascalemin (Variables|/Game/Gameplay/Parasite/PDA_ParasiteData.PDA_ParasiteData_C|GetExplosionNiagaraScaleMin _entityparasitedata_2))
  (bind _explosionniagarascalemax (Variables|/Game/Gameplay/Parasite/PDA_ParasiteData.PDA_ParasiteData_C|GetExplosionNiagaraScaleMax _entityparasitedata_2))
  (bind _returnvalue (Math|Float|MapRangeClamped _parasitelevel _parasitemin _parasitemax _explosionniagarascalemin _explosionniagarascalemax))
  (if (not (Variables|Data|GetExploding))
    (Variables|Data|SetExploding true)
    (if (Variables|/Game/Gameplay/Parasite/PDA_ParasiteData.PDA_ParasiteData_C|GetDebugDrawSpheres (Variables|Data|GetEntityParasiteData))
      (Rendering|Debug|DrawDebugSphere (Transformation|GetActorLocation (Components|GetOwner)) (Variables|/Game/Gameplay/Parasite/PDA_ParasiteData.PDA_ParasiteData_C|GetExplosionRadius (Variables|Data|GetEntityParasiteData)) 12 "(R=1.000000,G=0.830048,B=0.000000,A=1.000000)" 2.0 1.0))
    (bind _outcomponents (Collision|SphereOverlapComponents (Transformation|GetActorLocation (Components|GetOwner)) (Variables|/Game/Gameplay/Parasite/PDA_ParasiteData.PDA_ParasiteData_C|GetExplosionRadius (Variables|Data|GetEntityParasiteData)) (Utilities|Array|MakeArray "ObjectTypeQuery3" "ObjectTypeQuery2" "ObjectTypeQuery4" "ObjectTypeQuery10") 0 (Utilities|Array|MakeArray (Components|GetOwner))))
    (for _array_element _outcomponents
      (Utilities|IsValid _array_element
        (:Is%20Valid
          (Utilities|IsValid (Components|GetOwner _array_element)
            (:Is%20Valid
              (if (Physics|IsSimulatingPhysics _array_element "None")
                (Physics|AddImpulseatLocation _array_element (* (Variables|/Game/Gameplay/Parasite/PDA_ParasiteData.PDA_ParasiteData_C|GetPhysicsActorForceFactor (Variables|Data|GetEntityParasiteData)) (CallFunction|CalculateImpulseForce (Components|GetOwner _array_element))) (Transformation|GetActorLocation (Components|GetOwner)) "None")
                (else
                  (Utilities|IsValid (Actor|GetComponentbyClass (Components|GetOwner _array_element) "/Script/Engine.CharacterMovementComponent")
                    (:Is%20Valid
                      (if (Actor|ActorHasTag (Components|GetOwner _array_element) "Player")
                        (Physics|AddImpulse (Actor|GetComponentbyClass (Components|GetOwner _array_element) "/Script/Engine.CharacterMovementComponent") (Math|Vector|MakeVector (.x (* (CallFunction|CalculateImpulseForce (Components|GetOwner _array_element)) (Variables|/Game/Gameplay/Parasite/PDA_ParasiteData.PDA_ParasiteData_C|GetPawnsForceFactor _entityparasitedata))) (.y (* (CallFunction|CalculateImpulseForce (Components|GetOwner _array_element)) (Variables|/Game/Gameplay/Parasite/PDA_ParasiteData.PDA_ParasiteData_C|GetPawnsForceFactor _entityparasitedata))) (+ (.z (* (CallFunction|CalculateImpulseForce (Components|GetOwner _array_element)) (Variables|/Game/Gameplay/Parasite/PDA_ParasiteData.PDA_ParasiteData_C|GetPawnsForceFactor _entityparasitedata))) (Variables|/Game/Gameplay/Parasite/PDA_ParasiteData.PDA_ParasiteData_C|GetFixedVerticalForceOffset _entityparasitedata))) false)))))))))))
    (if (Variables|/Game/Gameplay/Parasite/PDA_ParasiteData.PDA_ParasiteData_C|GetDebugDrawSpheres (Variables|Data|GetEntityParasiteData))
      (Rendering|Debug|DrawDebugSphere (Transformation|GetActorLocation (Components|GetOwner)) (Variables|/Game/Gameplay/Parasite/PDA_ParasiteData.PDA_ParasiteData_C|GetKillRadius (Variables|Data|GetEntityParasiteData)) 12 "(R=1.000000,G=0.000000,B=0.010660,A=1.000000)" 2.0 1.0))
    (bind _outactors (Collision|SphereOverlapActors (Transformation|GetActorLocation (Components|GetOwner)) (Variables|/Game/Gameplay/Parasite/PDA_ParasiteData.PDA_ParasiteData_C|GetKillRadius (Variables|Data|GetEntityParasiteData)) (Utilities|Array|MakeArray "ObjectTypeQuery3" "ObjectTypeQuery2" "ObjectTypeQuery4" "ObjectTypeQuery10") 0 (Utilities|Array|MakeArray (Components|GetOwner))))
    (for _array_element_2 _outactors
      (Utilities|IsValid _array_element_2
        (:Is%20Valid
          (if (Actor|ActorHasTag _array_element_2 "Enemy")
            (if (!= _array_element_2 (CallFunction|GetPlayerGrabbedEntity))
              (Actor|DestroyActor _array_element_2)
              (elif (Actor|ActorHasTag _array_element_2 "Player")
                (bind _asbp_fps_character (Utilities|Casting|CastToBP_FPS_Character _array_element_2))
                (Default|ParasiteExplosion _asbp_fps_character)))))))
    (Niagara|SpawnSystematLocation (Variables|/Game/Gameplay/Parasite/PDA_ParasiteData.PDA_ParasiteData_C|GetExplosionNiagaraSystem _entityparasitedata_2) (Transformation|GetActorLocation (Components|GetOwner)) "0, 0, 0" (Math|Vector|MakeVector _returnvalue _returnvalue _returnvalue) true true "AutoRelease")
    (Default|CallExplosionTriggered)))

(event Custom|StartProcTimer
  (bind _returnvalue (Utilities|Time|SetTimerbyEvent (EventDispatchers|CreateEvent :!event Custom|TimerProc) (Variables|/Game/Gameplay/Parasite/PDA_ParasiteData.PDA_ParasiteData_C|GetParasiteProcDelay (Variables|Data|GetEntityParasiteData)) true))
  (Variables|Functional|SetParasiteTimer _returnvalue)
  (Development|PrintString "ParasiteStart"))

(event Custom|StopProcTimer
  (Utilities|Time|ClearandInvalidateTimerbyHandle (Variables|Functional|GetParasiteTimer)))

(event Custom|DelayedExplosion
  (Utilities|FlowControl|Delay (Variables|/Game/Gameplay/Parasite/PDA_ParasiteData.PDA_ParasiteData_C|GetExplosionDelay (Variables|Data|GetEntityParasiteData)))
  (CallFunction|Explosion))

(event Custom|TimerProc
  (CallFunction|ProcParasite)
  (if (not (< (Variables|Data|GetParasiteLevel) (Variables|/Game/Gameplay/Parasite/PDA_ParasiteData.PDA_ParasiteData_C|GetParasiteMax (Variables|Data|GetEntityParasiteData))))
    (CallFunction|Explosion)))

(event EventBeginPlay
  (if (Variables|Default|GetEnabled)
    (Components|Activation|Activate false)
    (else
      (Components|Activation|Deactivate))))

(fn UpdateParasiteMaterial
  (params (FullyCharged :type Boolean))
  (bind _parasitemid (Variables|Functional|GetParasiteMID))
  (Rendering|Material|SetScalarParameterValue _parasitemid "Line_Edge" (Variables|Data|GetParasiteLevel) :!class /Script/Engine.MaterialInstanceDynamic)
  (if FullyCharged
    (Rendering|Material|SetScalarParameterValue _parasitemid "Erosion" 15.0 :!class /Script/Engine.MaterialInstanceDynamic)))

(fn CalculateImpulseForce
  (params (TargetActor :type Actor%20Object%20Reference))
  (return (* (Math|Vector|Normalize (- (Transformation|GetActorLocation TargetActor) (Transformation|GetActorLocation (Components|GetOwner)))) (Variables|/Game/Gameplay/Parasite/PDA_ParasiteData.PDA_ParasiteData_C|GetExplosionForce (Variables|Data|GetEntityParasiteData)) (Variables|Data|GetParasiteLevel))))

(fn ConvertBulletstoParasite
  (bind _entityparasitedata (Variables|Data|GetEntityParasiteData))
  (bind _bulletstoexplode (Variables|/Game/Gameplay/Parasite/PDA_ParasiteData.PDA_ParasiteData_C|GetBulletsToExplode _entityparasitedata))
  (bind _returnvalue (Math|Conversions|ToFloat(Integer) _bulletstoexplode))
  (Variables|Data|SetParasiteLevel (Math|Float|MapRangeClamped (Math|Float|Clamp(Float) (Math|Conversions|ToFloat(Integer) (- (Variables|Data|GetBulletsTaken) 1)) 0.0 _returnvalue) 0.0 _returnvalue (Variables|/Game/Gameplay/Parasite/PDA_ParasiteData.PDA_ParasiteData_C|GetParasiteMin _entityparasitedata) (Variables|/Game/Gameplay/Parasite/PDA_ParasiteData.PDA_ParasiteData_C|GetParasiteMax _entityparasitedata))))

(fn AtMaxBulletStacks
  (return (>= (Variables|Data|GetBulletsTaken) (+ (Variables|/Game/Gameplay/Parasite/PDA_ParasiteData.PDA_ParasiteData_C|GetBulletsToExplode (Variables|Data|GetEntityParasiteData)) 1))))

(fn GetPlayerGrabbedEntity
  (bind _asbp_fps_character (Utilities|Casting|CastToBP_FPS_Character (Game|Player|GetPlayerPawn 0)))
  (Utilities|IsValid (Actor|GetComponentbyClass _asbp_fps_character "/Game/Gameplay/Player/BPC_Weapon.BPC_Weapon_C")
    (:Is%20Valid
      (Utilities|IsValid (.Actor (Utilities|Struct|BreakS_GrabbedEntity (Default|GetGrabbedEntity (Actor|GetComponentbyClass _asbp_fps_character "/Game/Gameplay/Player/BPC_Weapon.BPC_Weapon_C"))))
        (:Is%20Valid
          (return (.Actor (Utilities|Struct|BreakS_GrabbedEntity (Default|GetGrabbedEntity (Actor|GetComponentbyClass _asbp_fps_character "/Game/Gameplay/Player/BPC_Weapon.BPC_Weapon_C"))))))))))