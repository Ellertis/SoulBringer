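; BP_Timer is a timer actor that measures how long the player takes to get from a start trigger box to an end trigger box.
; Overlapping StartBox starts the count or resets it if already running, and EndBox stops it and stores the last time.
; Tick accumulates delta seconds, shows the current or last time via PrintString, and rotates two text renders using a look-at from the player with yaw flipped 180 degrees.
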(event OnComponentBeginOverlap(StartBox)
  (params (OverlappedComponent :type Primitive%20Component%20Object%20Reference) (OtherActor :type Actor%20Object%20Reference) (OtherComp :type Primitive%20Component%20Object%20Reference) (OtherBodyIndex :type Integer) (bFromSweep :type Boolean) (SweepResult :type Hit%20Result%20Structure%20%28by%20ref%29))
  (if (== OtherActor (Game|Player|GetPlayerPawn 0))
    (if (not (Variables|Default|GetActive))
      (Variables|Default|SetActive true)
      (else
        (Variables|Default|SetTime 0.0)))))

(event OnComponentBeginOverlap(EndBox)
  (params (OverlappedComponent :type Primitive%20Component%20Object%20Reference) (OtherActor :type Actor%20Object%20Reference) (OtherComp :type Primitive%20Component%20Object%20Reference) (OtherBodyIndex :type Integer) (bFromSweep :type Boolean) (SweepResult :type Hit%20Result%20Structure%20%28by%20ref%29))
  (if (== OtherActor (Game|Player|GetPlayerPawn 0))
    (if (Variables|Default|GetActive)
      (Variables|Default|SetActive false)
      (Variables|Default|SetLastTime (Variables|Default|GetTime))
      (Variables|Default|SetTime 0.0))))

(event EventBeginPlay)

(event Collision|EventActorBeginOverlap
  (params (OtherActor :type Actor%20Object%20Reference)))

(event EventTick
  (params (DeltaSeconds :type Float%20%28single-precision%29))
  (bind _returnvalue (Game|Player|GetPlayerPawn 0))
  (bind _textrender (Variables|Default|GetTextRender))
  (bind _textrender1 (Variables|Default|GetTextRender1))
  (bind _returnvalue_2 (Transformation|GetWorldLocation _textrender1))
  (bind _returnvalue_3 (Transformation|GetActorLocation _returnvalue))
  (bind _returnvalue_4 (Transformation|GetWorldLocation _textrender))
  (bind _returnvalue_5 (Math|Rotator|FindLookatRotation _returnvalue_3 _returnvalue_4))
  (bind _returnvalue_6 (Math|Rotator|FindLookatRotation _returnvalue_3 _returnvalue_2))
  (Transformation|SetWorldRotation (Variables|Default|GetTextRender) (Math|Rotator|MakeRotator (.roll _returnvalue_5) (.pitch _returnvalue_5) (+ (.yaw _returnvalue_5) 1.8e+02)) false false)
  (Transformation|SetWorldRotation (Variables|Default|GetTextRender1) (Math|Rotator|MakeRotator (.roll _returnvalue_6) (.pitch _returnvalue_6) (+ (.yaw _returnvalue_6) 1.8e+02)) false false)
  (if (Variables|Default|GetActive)
    (Variables|Default|SetTime (+ (Variables|Default|GetTime) (Utilities|Time|GetWorldDeltaSeconds)))
    (Development|PrintString (Utilities|String|Append "Current Time : " (Utilities|String|ToString(Float) (Variables|Default|GetTime))) true false "(R=0.000000,G=0.660000,B=1.000000,A=1.000000)" 0.001)
    (else
      (Development|PrintString (Utilities|String|Append "Last Time : " (Utilities|String|ToString(Float) (Variables|Default|GetLastTime))) true false "(R=0.000000,G=0.660000,B=1.000000,A=1.000000)" 0.001))))

(fn ConstructionScript)