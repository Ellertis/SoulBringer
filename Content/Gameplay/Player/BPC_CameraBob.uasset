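; Player component that adds Quake-style head bob to the camera and weapon mesh while the owner moves.
; One tick after BeginPlay, if enabled with a valid camera, it stores both starting locations and starts a looping CameraBob timer, otherwise it deactivates.
; CameraBob advances a wrapped phase and applies sine and absolute-cosine offsets to those locations, scaled by the owner's squared velocity against a maximum.
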(event EventBeginPlay
  (Utilities|FlowControl|DelayUntilNextTick)
  (if (and (Variables|Default|GetEnabled) (Utilities|IsValid (Variables|Default|GetCameraRef)))
    (Components|Activation|Activate false)
    (Variables|Default|SetCameraStartLoc (Variables|/Script/Engine.SceneComponent|GetRelativeLocation (Variables|Default|GetCameraRef)))
    (Variables|Default|SetWeaponStartLoc (Variables|/Script/Engine.SceneComponent|GetRelativeLocation (Variables|Default|GetWeaponMesh)))
    (bind _returnvalue (Utilities|Time|SetTimerbyFunctionName 0 "CameraBob" (Variables|Default|GetDeltaTime) true))
    (Variables|Default|SetBobTimer _returnvalue)
    (else
      (Components|Activation|Deactivate))))

(fn CameraBob
  (bind _returnvalue (Components|GetOwner))
  (bind _maxvelocitysquared (Variables|Default|GetMaxVelocitySquared))
  (bind _returnvalue_2 (Transformation|GetVelocity _returnvalue))
  (bind _returnvalue_3 (Math|Vector|VectorLengthSquared _returnvalue_2))
  (bind _returnvalue_4 (Math|Float|MapRangeClamped _returnvalue_3 0.0 _maxvelocitysquared 0.0 1.0))
  (bind _output_get (Variables|Default|SetBobTime (Math|Float|%(Float) (+ (Variables|Default|GetBobTime) (* (Variables|Default|GetDeltaTime) (Variables|Default|GetBobFrequency))) 6.283186)))
  (Transformation|SetRelativeLocation (Variables|Default|GetCameraRef) (+ (Variables|Default|GetCameraStartLoc) (Math|Vector|MakeVector (* (Math|Trig|Sin(Radians) _output_get) (Variables|Default|GetSideBobAmplitude) _returnvalue_4) 0.0 (Math|Float|Absolute(Float) (* (Math|Trig|Cos(Radians) _output_get) (Variables|Default|GetVerticalBobAmplitude) _returnvalue_4)))) false false)
  (Transformation|SetRelativeLocation (Variables|Default|GetWeaponMesh) (+ (Variables|Default|GetWeaponStartLoc) (Math|Vector|MakeVector (Math|Float|Absolute(Float) (* (Math|Trig|Cos(Radians) _output_get) 4.0 _returnvalue_4)) 0.0 0.0)) false false)
  (if (Math|Float|NearlyEqual(Float) _returnvalue_3 0.0 0.02)
    _))