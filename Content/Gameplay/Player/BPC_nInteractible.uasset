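; Player component that picks which overlapping BP_ShooterPickup the camera is aimed at.
; Each tick it scores every pickup by the dot product of camera forward and the owner-to-pickup direction.
; When the best score exceeds a threshold, that pickup's ShowUI is set and it becomes CurrentTarget; neither is cleared here.
; The best-scoring actor's name prints every tick as debug output.
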(event EventBeginPlay)

(event EventTick
  (params (DeltaSeconds :type Float%20%28single-precision%29))
  (bind _returnvalue (Components|GetOwner))
  (bind _floatvalues (Variables|Default|GetFloatValues))
  (bind _overlappingactors (Collision|GetOverlappingActors _returnvalue "/Game/Variant_Shooter/Blueprints/Pickups/BP_ShooterPickup.BP_ShooterPickup_C" :!class /Script/Engine.Actor))
  (bind (_indexofmaxvalue _maxvalue) (Math|Float|MaxOfFloatArray _floatvalues))
  (bind _output (Utilities|Array|Get(acopy) _overlappingactors _indexofmaxvalue))
  (Utilities|Array|Clear (Variables|Default|GetFloatValues))
  (for (_array_element _array_index) _overlappingactors
    (Utilities|Array|SetArrayElem (Variables|Default|GetFloatValues) _array_index (Math|Vector|DotProduct (Math|Vector|GetForwardVector (Variables|Default|GetCameraRef)) (Math|Vector|Normalize (- (Transformation|GetActorLocation _array_element) (Transformation|GetActorLocation (Components|GetOwner))))) true))
  (Development|PrintString (Utilities|String|Append "Closest Actor  DOT IS " (Utilities|GetDisplayName _output)) true false "(R=0.000000,G=0.660000,B=1.000000,A=1.000000)" 0.001)
  (if (> _maxvalue 0.8)
    (Variables|/Game/Variant_Shooter/Blueprints/Pickups/BP_ShooterPickup.BP_ShooterPickup_C|SetShowUI _output true)
    (Variables|Default|SetCurrentTarget _output)))