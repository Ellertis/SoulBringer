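; Player actor component that rolls the first player controller's control rotation to lean the camera during movement.
; TriggerLean stores the movement axis value, which sets the lean direction, and resumes a paused looping timer.
; The timer-driven Lean function interpolates roll toward an angle mapped from squared owner speed, preserving pitch and yaw.
; With zero input and near-level roll, it snaps roll to zero and pauses the timer.
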(event Custom|TriggerLean
  (params (MovementAxisValue :type Float%20%28double-precision%29))
  (bind _leantimer (Variables|Default|GetLeanTimer))
  (bind _output_get (Variables|Default|SetMovementAxisValue MovementAxisValue))
  (if (and (!= _output_get 0.0) (Class|KismetSystemLibrary|IsTimerPausedHandle _leantimer))
    (Utilities|Time|UnpauseTimerbyHandle _leantimer)))

(event EventBeginPlay
  (if (Variables|Default|GetEnabled)
    (Components|Activation|Activate false)
    (bind _returnvalue (Utilities|Time|SetTimerbyFunctionName 0 "Lean" (Variables|Default|GetDeltaTime) true))
    (Variables|Default|SetLeanTimer _returnvalue)
    (else
      (Components|Activation|Deactivate))))

(fn Lean
  (bind _returnvalue (Game|GetPlayerController 0))
  (bind _returnvalue_2 (Game|GetPlayerController 0))
  (bind _returnvalue_3 (Pawn|GetControlRotation _returnvalue_2 :!class /Script/Engine.Controller))
  (bind _returnvalue_4 (Pawn|GetControlRotation _returnvalue :!class /Script/Engine.Controller))
  (bind (_roll _pitch _yaw) (Math|Rotator|BreakRotator _returnvalue_4))
  (Pawn|SetControlRotation _returnvalue (Math|Interpolation|RInterpTo _returnvalue_4 (Math|Rotator|MakeRotator (* (Math|Float|MapRangeClamped (Math|Vector|VectorLengthSquared (Transformation|GetVelocity (Components|GetOwner))) 0.0 (Variables|Default|GetMaxVelocitySquarred) 0.0 (Variables|Default|GetLeanAngle)) (Math|Float|Sign(Float) (Variables|Default|GetMovementAxisValue))) _pitch _yaw) (Variables|Default|GetDeltaTime) (Variables|Default|GetLeanSpeed)))
  (if (and (Math|Float|NearlyEqual(Float) _roll 0.0 0.02) (== (Variables|Default|GetMovementAxisValue) 0.0))
    (Utilities|Time|PauseTimerbyHandle (Variables|Default|GetLeanTimer))
    (Pawn|SetControlRotation _returnvalue_2 (Math|Rotator|MakeRotator 0.0 (.pitch _returnvalue_3) (.yaw _returnvalue_3)))))