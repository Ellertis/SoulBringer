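; Player weapon component with automatic bullet fire and a gravity-gun style alt fire, driven by GunData.
; A looping timer fires bullets with additive, clamped spread that also scales camera shake and shot pitch.
; Each shot kicks controller pitch, softened from the tenth shot, and Tick recovers it.
; Alt fire launches a grenade whose hit callback grabs the target with a PhysicsHandle; the next alt fire hurls it forward.
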(event Custom|Fire
  (bind _gundata (Variables|Default|GetGunData))
  (bind _projectilespawnpoint (Variables|Components|GetProjectileSpawnPoint))
  (bind _gundata_2 (Variables|Default|GetGunData))
  (bind _returnvalue (Transformation|GetWorldLocation _projectilespawnpoint))
  (bind _gundata_3 (Variables|/Game/Gameplay/Player/WeaponsData/PDA_WeaponData.PDA_WeaponData_C|GetGunData _gundata_2))
  (bind _gundata_4 (Variables|/Game/Gameplay/Player/WeaponsData/PDA_WeaponData.PDA_WeaponData_C|GetGunData _gundata))
  (bind (_accuracyvariationfactor _accuracymin _accuracymax) (Utilities|Struct|BreakS_WeaponData _gundata_3))
  (bind (_leftclickprojectilevelocty _leftclicklifespan _leftclickdamage _leftclickgravityscale) (Utilities|Struct|BreakS_WeaponData _gundata_4))
  (Math|Integer|IncrementInt (Variables|Default|GetShotCount)
    (:%20%20
      (Game|SpawnActorfromClass "/Game/Variant_Shooter/Blueprints/Pickups/Projectiles/BP_ShooterProjectile_Bullet.BP_ShooterProjectile_Bullet_C" (Math|Transform|MakeTransform _returnvalue (Math|Rotator|FindLookatRotation _returnvalue (+ _returnvalue (Math|Vector|GetForwardVector _projectilespawnpoint) (* (Math|Random|RandomUnitVector) (Variables|Default|GetCurrAccuracyVariance)))) "1.000000,1.000000,1.000000") "AlwaysSpawn" "MultiplyWithRoot" 0 false _leftclickprojectilevelocty _leftclicklifespan _leftclickdamage _leftclickgravityscale (.AsPawn (Utilities|Casting|CastToPawn (Components|GetOwner))))
      (bind _output_get (Variables|Default|SetCurrAccuracyVariance (Math|Float|Clamp(Float) (+ (Variables|Default|GetCurrAccuracyVariance) (- _accuracyvariationfactor 1.0)) _accuracymin _accuracymax)))
      (CameraShakes|StartCameraShake (Game|GetPlayerCameraManager 0) (Variables|/Game/Gameplay/Player/WeaponsData/PDA_WeaponData.PDA_WeaponData_C|GetRecoilCameraShake (Variables|Default|GetGunData)) (Math|Float|MapRangeClamped _output_get _accuracymin _accuracymax 0.0 1.0) "CameraLocal" "0, 0, 0")
      (Audio|PlaySound2D (Variables|/Game/Gameplay/Player/WeaponsData/PDA_WeaponData.PDA_WeaponData_C|GetShotSoundCue (Variables|Default|GetGunData)) 1.0 (Math|Float|MapRangeClamped _output_get _accuracymin _accuracymax 0.6 1.0) 0.0 0 0 false)
      (Niagara|SpawnSystemAttached "/Game/Gameplay/Player/WeaponsData/NS_MuzzleFlash.NS_MuzzleFlash" (Variables|Components|GetProjectileSpawnPoint) "None" "0, 0, 0" "0, 0, 0" "SnapToTarget" true true "AutoRelease")
      (Utilities|FlowControl|Delay (Utilities|Operators|Divide 1.0 (.Firerate (Utilities|Struct|BreakS_WeaponData (Variables|/Game/Gameplay/Player/WeaponsData/PDA_WeaponData.PDA_WeaponData_C|GetGunData (Variables|Default|GetGunData)))) 1.5))
      (CallFunction|ApplyRecoil 1.0))))

(event Custom|TriggerFire
  (bind _firetimer (Variables|Default|GetFireTimer))
  (Variables|Default|SetCurrAccuracyVariance (.AccuracyMin (Utilities|Struct|BreakS_WeaponData (Variables|/Game/Gameplay/Player/WeaponsData/PDA_WeaponData.PDA_WeaponData_C|GetGunData (Variables|Default|GetGunData)))))
  (CallFunction|Fire)
  (Utilities|Time|ClearandInvalidateTimerbyHandle _firetimer)
  (CallFunction|SetFireTimer)
  (Utilities|Time|UnpauseTimerbyHandle _firetimer))

(event Custom|StopFire
  (Utilities|Time|ClearandInvalidateTimerbyHandle (Variables|Default|GetFireTimer)))

(event Custom|AltFire
  (bind _projectilespawnpoint (Variables|Components|GetProjectileSpawnPoint))
  (bind _gundata (Variables|Default|GetGunData))
  (bind _returnvalue (Transformation|GetWorldLocation _projectilespawnpoint))
  (bind _gundata_2 (Variables|/Game/Gameplay/Player/WeaponsData/PDA_WeaponData.PDA_WeaponData_C|GetGunData _gundata))
  (bind (_rightclickprojectilevelocty _rigthclicklifespan _rightclickdamage _rightclickgravityscale) (Utilities|Struct|BreakS_WeaponData _gundata_2))
  (Utilities|IsValid (.Actor (Utilities|Struct|BreakS_GrabbedEntity (Variables|Default|GetGrabbedEntity)))
    (:Is%20Valid
      (Physics|Components|PhysicsHandle|ReleaseComponent (Variables|Components|GetPhysicsHandle))
      (Physics|SetPhysicsLinearVelocity (.HitComponent (Utilities|Struct|BreakS_GrabbedEntity (Variables|Default|GetGrabbedEntity))) (* (Math|Vector|GetForwardVector (Variables|Components|GetProjectileSpawnPoint)) (.RightClickObjectForceProjection (Utilities|Struct|BreakS_WeaponData (Variables|/Game/Gameplay/Player/WeaponsData/PDA_WeaponData.PDA_WeaponData_C|GetGunData (Variables|Default|GetGunData))))) false "None")
      (Class|BPIGrabbable|OnPushObject(Message) (.Actor (Utilities|Struct|BreakS_GrabbedEntity (Variables|Default|GetGrabbedEntity))))
      (Variables|Default|SetGrabbedEntity "")
      (Utilities|Time|ClearandInvalidateTimerbyHandle (Variables|Default|GetPhysicsObjectTimer)))
    (:Is%20Not%20Valid
      (bind _returnvalue_2 (Game|SpawnActorfromClass "/Game/Variant_Shooter/Blueprints/Pickups/Projectiles/BP_ShooterProjectile_Grenade.BP_ShooterProjectile_Grenade_C" (Math|Transform|MakeTransform _returnvalue (Math|Rotator|FindLookatRotation _returnvalue (+ _returnvalue (Math|Vector|GetForwardVector _projectilespawnpoint) (* (Math|Random|RandomUnitVector) (Utilities|Struct|BreakS_WeaponData (Variables|/Game/Gameplay/Player/WeaponsData/PDA_WeaponData.PDA_WeaponData_C|GetGunData (Variables|Default|GetGunData)))))) "1.000000,1.000000,1.000000") "AlwaysSpawn" "MultiplyWithRoot" 0 _rightclickprojectilevelocty _rigthclicklifespan _rightclickdamage _rightclickgravityscale (.AsPawn (Utilities|Casting|CastToPawn (Components|GetOwner)))))
      (EventDispatchers|AssignHitActor _returnvalue_2 (EventDispatchers|CreateEvent :!event Custom|HitActor_Event)))))

(event Custom|SetPhysicsHandleLocation
  (bind _projectilespawnpoint (Variables|Components|GetProjectileSpawnPoint))
  (Physics|Components|PhysicsHandle|SetTargetLocation (Variables|Components|GetPhysicsHandle) (+ (Transformation|GetWorldLocation _projectilespawnpoint) (* (Math|Vector|GetForwardVector _projectilespawnpoint) (Variables|Default|GetHandleLength)) (* (* (Math|Vector|GetRightVector _projectilespawnpoint) -1.0) 1e+02))))

(event Custom|HitActor_Event
  (params (TargetActor :type Actor%20Object%20Reference) (HitComponent :type Primitive%20Component%20Object%20Reference))
  (Class|BPIGrabbable|OnPullObject(Message) TargetActor)
  (Physics|Components|PhysicsHandle|GrabComponentatLocationwithRotation (Variables|Components|GetPhysicsHandle) HitComponent "None" (Transformation|GetWorldLocation HitComponent) "0, 0, 0")
  (bind _output_get (Variables|Default|SetGrabbedEntity (Utilities|Struct|MakeS_GrabbedEntity TargetActor HitComponent)))
  (Variables|Default|SetHandleLength (* (Math|Vector|GetMaxElement (.BoxExtent (Collision|GetComponentBounds (Utilities|Struct|BreakS_GrabbedEntity _output_get)))) 2.5))
  (bind _returnvalue (Utilities|Time|SetTimerbyEvent (delegate Custom|SetPhysicsHandleLocation) 0.016 true))
  (Variables|Default|SetPhysicsObjectTimer _returnvalue))

(event Custom|SetFireTimer
  (bind _returnvalue (Utilities|Time|SetTimerbyEvent (delegate Custom|Fire) (/ 1.0 (.Firerate (Utilities|Struct|BreakS_WeaponData (Variables|/Game/Gameplay/Player/WeaponsData/PDA_WeaponData.PDA_WeaponData_C|GetGunData (Variables|Default|GetGunData))))) true))
  (bind _output_get (Variables|Default|SetFireTimer _returnvalue))
  (Utilities|Time|PauseTimerbyHandle _output_get)
  (Variables|Default|SetShotCount 0))

(event EventBeginPlay)

(event EventTick
  (params (DeltaSeconds :type Float%20%28single-precision%29))
  (CallFunction|RecoilRecovery))

(fn RecoilRecovery
  (bind _output_get (Variables|Default|SetAccumulatedRecoil (Math|Interpolation|FInterptoConstant (Variables|Default|GetAccumulatedRecoil) 0.0 (Utilities|Time|GetWorldDeltaSeconds) (.RecoilRecoverySpeed (Utilities|Struct|BreakS_WeaponData (Variables|/Game/Gameplay/Player/WeaponsData/PDA_WeaponData.PDA_WeaponData_C|GetGunData (Variables|Default|GetGunData)))))))
  (Pawn|Input|AddControllerPitchInput (Game|Player|GetPlayerPawn 0) (- _output_get (Math|Interpolation|FInterptoConstant (Variables|Default|GetAccumulatedRecoil) 0.0 (Utilities|Time|GetWorldDeltaSeconds) (.RecoilRecoverySpeed (Utilities|Struct|BreakS_WeaponData (Variables|/Game/Gameplay/Player/WeaponsData/PDA_WeaponData.PDA_WeaponData_C|GetGunData (Variables|Default|GetGunData))))))))

(fn ApplyRecoil
  (params (Scale :type Float%20%28double-precision%29))
  (bind _gundata (Variables|Default|GetGunData))
  (bind _gundata_2 (Variables|/Game/Gameplay/Player/WeaponsData/PDA_WeaponData.PDA_WeaponData_C|GetGunData _gundata))
  (bind (_recoilkickbackretentionfactor _recoilkickback _recoilrotationdegrees) (Utilities|Struct|BreakS_WeaponData _gundata_2))
  (Variables|Default|SetAccumulatedRecoil (+ (* (Variables|Default|GetAccumulatedRecoil) 0.5) _recoilkickback))
  (Pawn|Input|AddControllerPitchInput (Game|Player|GetPlayerPawn 0) (* _recoilkickback -1.0 (Math|Float|SelectFloat 0.7 1.0 (>= (Variables|Default|GetShotCount) 10)))))