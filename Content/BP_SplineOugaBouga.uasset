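; Spline-following actor that moves a budgeted skeletal mesh along its spline in a continuous loop over a set Duration.
; BeginPlay places the mesh at the start and caches its world scale, then starts a looping 0.016-second timer in place of Tick.
; MoveAlongSpline samples the spline at elapsed time modulo Duration, adds a rotation offset and advances time by a fixed step.
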(event Custom|MoveAlongSpline
  (Transformation|SetWorldTransform (Variables|Default|GetSkeletalMeshComponentBudgeted) (Math|Transform|MakeTransform (.Location (Math|Transform|BreakTransform (CallFunction|GetPointAlongSpline))) (Math|Rotator|CombineRotators (Class|SplineComponent|GetRotationatTime (Variables|Default|GetSpline) (Math|Float|%(Float) (Variables|Default|GetCurrDuration) (Variables|Default|GetDuration)) "World" false) (Math|Conversions|RotationFromXVector (Variables|Default|GetRotationOffset))) (Variables|Default|GetScaleOffset)) false false)
  (Variables|Default|SetCurrDuration (+ (Variables|Default|GetCurrDuration) 0.016)))

(event EventBeginPlay
  (bind _transform (CallFunction|GetPointAlongSpline))
  (bind (_location _rotation) (Math|Transform|BreakTransform _transform))
  (Variables|/Script/Engine.SplineComponent|SetDuration (Variables|Default|GetSpline) (Variables|Default|GetDuration))
  (Variables|Default|SetScaleOffset (Transformation|GetWorldScale (Variables|Default|GetSkeletalMeshComponentBudgeted)))
  (Transformation|SetWorldTransform (Variables|Default|GetSkeletalMeshComponentBudgeted) (Math|Transform|MakeTransform _location (Math|Conversions|RotationFromXVector (+ _rotation (Variables|Default|GetRotationOffset))) (Variables|Default|GetScaleOffset)) false false)
  (bind _returnvalue (Utilities|Time|SetTimerbyEvent (EventDispatchers|CreateEvent :!event Custom|MoveAlongSpline) 0.016 true))
  (Variables|Default|SetMoveTimer _returnvalue))

(event Collision|EventActorBeginOverlap
  (params (OtherActor :type Actor%20Object%20Reference)))

(event EventTick
  (params (DeltaSeconds :type Float%20%28single-precision%29)))

(fn ConstructionScript)

(fn GetPointAlongSpline
  (return (Spline|GetTransformatTime (Variables|Default|GetSpline) (Math|Float|%(Float) (Variables|Default|GetCurrDuration) (Variables|Default|GetDuration)) "World" false false)))