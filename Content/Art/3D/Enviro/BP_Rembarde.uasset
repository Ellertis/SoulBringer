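; Railing environment prop that builds a repeatable row of pillars and small railing sections along local Y from a segment count.
; The construction script adds instanced static meshes at per-part offsets, with an optional closing pillar at the end.
; Each pillar is drawn from one of four variant instanced mesh components using a seeded random stream, while railing sections share a single component.
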(event Custom|RandomizePillarMaterials)

(event EventBeginPlay)

(event Collision|EventActorBeginOverlap
  (params (OtherActor :type Actor%20Object%20Reference)))

(event EventTick
  (params (DeltaSeconds :type Float%20%28single-precision%29)))

(fn ConstructionScript
  (for _index (range 0 (- (Variables|Default|GetCount) 1))
    (Components|InstancedStaticMesh|AddInstance (CallFunction|GetRandomPillarISM) (Math|Transform|MakeTransform (Math|Vector|MakeVector 0.0 (* _index (Variables|Default|GetPilarOffset)) 0.0) "0, 0, 0" "1.000000,1.000000,1.000000") false)
    (Components|InstancedStaticMesh|AddInstance (Variables|Default|GetSmallRembard_ISM) (Math|Transform|MakeTransform (Math|Vector|MakeVector 0.0 (* _index (Variables|Default|GetRembardOffset)) 0.0) "0, 0, 0" "1.000000,1.000000,1.000000") false))
  (if (Variables|Default|GetEndPillier)
    (Components|InstancedStaticMesh|AddInstance (CallFunction|GetRandomPillarISM) (Math|Transform|MakeTransform (Math|Vector|MakeVector 0.0 (* (Variables|Default|GetCount) (Variables|Default|GetPilarOffset)) 0.0) "0, 0, 0" "1.000000,1.000000,1.000000") false)))

(fn GetRandomPillarISM
  (return (.OutItem (Utilities|Array|RandomFromStream (Utilities|Array|MakeArray (Variables|Default|GetPillar_ISM) (Variables|Default|GetPillar_ISMVar2) (Variables|Default|GetPillar_ISMVar3) (Variables|Default|GetPillar_ISMVar4)) (Variables|Default|GetSeed)))))