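; Level streaming trigger actor that asynchronously loads and shows a soft-referenced level when a player-controlled pawn enters its box, and unloads it on exit.
; With Preload set, BeginPlay requests a hidden load, then immediately calls the visible load too, without waiting for overlap.
; Preload, load and unload are separate non-blocking events, each followed by its own finished notification.
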(event Custom|OnBoxBeginOverlap
  (params (OverlappedComponent :type Primitive%20Component%20Object%20Reference) (OtherActor :type Actor%20Object%20Reference) (OtherComp :type Primitive%20Component%20Object%20Reference) (OtherBodyIndex :type Integer) (bFromSweep :type Boolean) (SweepResult :type Hit%20Result%20Structure%20%28by%20ref%29))
  (if (CallFunction|IsPlayer OtherActor)
    (CallFunction|LoadLevel (Variables|Default|GetLevelToLoad))))

(event Custom|OnBoxEndOverlap
  (params (OverlappedComponent :type Primitive%20Component%20Object%20Reference) (OtherActor :type Actor%20Object%20Reference) (OtherComp :type Primitive%20Component%20Object%20Reference) (OtherBodyIndex :type Integer))
  (if (CallFunction|IsPlayer OtherActor)
    (CallFunction|UnloadLevel (Variables|Default|GetLevelToLoad))))

(event Custom|Load%20Level
  (params (Level :type World%20Soft%20Object%20Reference))
  (Class|GameplayStatics|LoadStreamLevelbySoftObjectPtr Level true false)
  (Default|CallLoadingFinished))

(event Custom|Preload%20Level
  (params (Level :type World%20Soft%20Object%20Reference))
  (Class|GameplayStatics|LoadStreamLevelbySoftObjectPtr Level false false)
  (Default|CallPreloadingFinished))

(event Custom|Unload%20Level
  (params (Level :type World%20Soft%20Object%20Reference))
  (Class|GameplayStatics|UnloadStreamLevelbySoftObjectPtr Level false)
  (Default|CallUnloadingFinished))

(event EventBeginPlay
  (bind _box (Variables|Default|GetBox))
  (bind _leveltoload (Variables|Default|GetLevelToLoad))
  (Collision|BindEventtoOnComponentBeginOverlap _box (EventDispatchers|CreateEvent :!event Custom|OnBoxBeginOverlap))
  (Collision|BindEventtoOnComponentEndOverlap _box (EventDispatchers|CreateEvent :!event Custom|OnBoxEndOverlap))
  (if (Variables|Default|GetPreload)
    (CallFunction|PreloadLevel _leveltoload)
    (CallFunction|LoadLevel _leveltoload)))

(fn ConstructionScript)

(fn IsPlayer
  (params (Object :type Object%20Object%20Reference))
  (bind _aspawn (Utilities|Casting|CastToPawn Object)
    (:then
      _)
    (:CastFailed
      _))
  (return (Pawn|IsPlayerControlled _aspawn)))